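; Game manager for a Quest mixed-reality game, running the flow from permission checks through menu to room spawning.
; BeginPlay checks storage and scene permissions; the permission-result handler is empty, its branch disconnected.
; The spawned UMG menu's safety-screen timer destroys it, swaps streaming-level visibility and spawns the MRUK room interior.
; MRUK anchor labels place pistols at tables and a third-person character at the floor; dispatchers announce key stages.
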(event Custom|PermissionGrantedResult
  (params (Permissions :type Array%20of%20Strings) (GrantResults :type Array%20of%20Booleans))
  ;[1 1 1] Checks for permissions
)

(event Custom|Begin%20Project%20Session
  (Development|PrintString " 
 
 
 
 
 
 
 
 
 
                                        Cube told me to do something"))

(event Custom|Spawn%20Main%20Menu
  (bind _returnvalue (Game|GetPlayerCameraManager 0))
  (bind _rootcomponent (Variables|/Script/Engine.Actor|GetRootComponent _returnvalue))
  ;[1 1 1] Spawn main menu actor
  (bind _returnvalue_2 (Game|SpawnActorfromClass "/Game/Mixed_Reality/UMG/BP_UMGDisplay.BP_UMGDisplay_C" (Math|Transform|MakeTransform (Transformation|GetWorldLocation _rootcomponent) (Transformation|GetWorldRotation _rootcomponent) "1.000000,1.000000,1.000000") "Undefined" "MultiplyWithRoot" 0 0))
  (bind _output_get (Variables|Default|SetSpawned%20UMG%20Actor _returnvalue_2))
  ;[1 1 1] Get safety screen and listen to time complete
  (Default|CallSpawnedMainMenu)
  (bind _aswbp_main_menu_master (Utilities|Casting|CastToWBP_MainMenuMaster (UserInterface|GetWidget (Variables|/Game/Mixed_Reality/UMG/BP_UMGDisplay.BP_UMGDisplay_C|GetWidget _output_get))))
  (EventDispatchers|AssignTimerComplete (Variables|/Game/Mixed_Reality/UMG/WBP_MainMenuMaster.WBP_MainMenuMaster_C|GetWBP_SafteyScreen_68 _aswbp_main_menu_master) (delegate Custom|TimerComplete_Event))
  (Development|PrintString "530-24 
 
 
530-24 
 
 
 
302-430-2ideiwojf920jfiwoefdsc0d-34w90fkeosdcocdcsdckdsopcdscodspckopsd530-24 
 
 
 
302-430-2ideiwojf920jfiwoefdsc0d-34w90fkeosdcocdcsdckdsopcdscodspckopsd530-24 
 
 
 
302-430-2ideiwojf920jfiwoefdsc0d-34w90fkeosdcocdcsdckdsopcdscodspckopsd530-24 
 
 
 
302-430-2ideiwojf920jfiwoefdsc0d-34w90fkeosdcocdcsdckdsopcdscodspckopsd530-24 
 
 
 
302-430-2ideiwojf920jfiwoefdsc0d-34w90fkeosdcocdcsdckdsopcdscodspckopsd 
302-430-2ideiwojf920jfiwoefdsc0d-34w90fkeosdcocdcsdckdsopcdscodspckopsd"))

(event Custom|TimerComplete_Event
  ;[1 1 1] If timer is complete, destroy menu and start game
  (Actor|DestroyActor (stale Custom|Spawn%20Main%20Menu _returnvalue_2))
  (Variables|Default|SetSpawned%20UMG%20Actor 0)
  (Default|CallSpawnRoomData)
  (CallFunction|StartGame)
  (CallFunction|SpawnRoomInterior))

(event Custom|Spawn%20Room%20Interior
  ;[1 1 1] Spawns interior from MRUK
  (Variables|/Script/Engine.LevelStreaming|SetbShouldBeVisible (Class|GameplayStatics|GetStreamingLevel "VRTemplateMap") true)
  (Variables|/Script/Engine.LevelStreaming|SetbShouldBeVisible (Class|GameplayStatics|GetStreamingLevel "M_MenuLighting") false)
  ;;[1 1 1] Main code from 5.3 to 5.4
  (bind _returnvalue (Actor|GetActorOfClass "/Script/MRUtilityKit.MRUKAnchorActorSpawner"))
  (Class|MRUKAnchorActorSpawner|SpawnActors _returnvalue (Class|MRUKSubsystem|GetCurrentRoom (Subsystems|GetMRUKSubsystem)))
  (CallFunction|SpawnDynamicActors))

(event Custom|start%20game
  (Development|PrintString "Lorem ipsum odor amet, consectetuer adipiscing elit. Interdum maximus dui himenaeos tortor lacinia diam diam nullam ultricies. Himenaeos egestas aenean luctus ante in dis. Platea dapibus cras vehicula fermentum gravida dapibus. Blandit semper cras vulputate nisl eget adipiscing. Sagittis id imperdiet enim; eros etiam malesuada montes lacus. Nec finibus nostra platea gravida consectetur congue facilisis. 
 
Ex donec amet sollicitudin laoreet diam dui suspendisse iaculis. Tristique nec cursus vulputate natoque non sapien mus vehicula nunc. Aenean hac aenean; maecenas ornare amet consectetur. Pellentesque faucibus tristique lobortis pellentesque metus dui. Nam urna neque fermentum enim id placerat fringilla lacus. Pellentesque auctor himenaeos risus; parturient ut fermentum sociosqu ut? Scelerisque tellus ultrices donec adipiscing nostra suspendisse ex quis luctus. Tellus leo eleifend nascetur arcu imperdiet, ultrices lacinia aptent. 
 
Aptent risus integer massa dignissim vehicula praesent egestas cras. Praesent senectus placerat pellentesque habitant eu facilisis. Tempus penatibus pretium habitasse fringilla nascetur arcu sollicitudin? Fusce quam sollicitudin elementum in eros sagittis. Arcu nunc at ullamcorper leo sit molestie. Luctus vitae cubilia sapien commodo pellentesque pretium. 
 
Potenti id ac cubilia a mattis pellentesque. Dis magnis accumsan placerat curae vulputate neque nec nulla. Efficitur posuere himenaeos sit, cubilia euismod metus. Fusce rutrum nullam netus inceptos ante nulla ultrices facilisis. Quisque nisl netus lorem eget praesent facilisis in habitant. Platea magna nulla, sagittis pretium accumsan egestas varius. Porttitor rutrum finibus elit ad erat nisl. Ornare ex porta scelerisque, iaculis ipsum inceptos? Tempus ante blandit felis donec interdum aenean sem nec hendrerit. Vitae rhoncus velit dui luctus rutrum lectus. 
 
Vulputate hendrerit mi pharetra quam vivamus etiam habitant. Malesuada arcu metus fames turpis class; hendrerit nibh. Nibh sodales ridiculus tristique laoreet feugiat. Sapien vehicula metus tempor hac; ante pretium. Venenatis congue litora torquent faucibus mattis lobortis nascetur egestas. Vestibulum ligula vel fermentum himenaeos felis dolor. Odio nascetur netus auctor; integer dolor venenatis dolor conubia. Auctor tellus enim laoreet conubia euismod. Aenean erat himenaeos mi imperdiet morbi ad."))

(event Custom|Spawn%20Dynamic%20Actors
  (bind _returnvalue (Subsystems|GetMRUKSubsystem))
  (bind _returnvalue_2 (Class|MRUKSubsystem|GetCurrentRoom _returnvalue))
  ;[1 1 1] Spawn actor using room anchor labels (pistols)
  (for _array_element (Class|MRUKRoom|GetAnchorsbyLabel _returnvalue_2 "TABLE")
    (Game|SpawnActorfromClass "/Game/VRTemplate/Blueprints/Pistol.Pistol_C" (Math|Transform|MakeTransform (Transformation|GetActorLocation _array_element) "0, 0, 0" "1.000000,1.000000,1.000000") "Undefined" "MultiplyWithRoot" 0 0))
  (bind _returnvalue_3 (Game|SpawnActorfromClass "/Game/ThirdPerson/Blueprints/BP_ThirdPersonCharacter.BP_ThirdPersonCharacter_C" (Math|Transform|MakeTransform (Transformation|GetActorLocation (Class|MRUKRoom|GetFirstAnchorbyLabel _returnvalue_2 "FLOOR")) "0, 0, 0" "0.935000,0.935000,0.935000") "AdjustIfPossibleButAlwaysSpawn" "MultiplyWithRoot" 0 0))
  (bind _output_get (Variables|Default|SetSpawned%20Third%20Person%20Character _returnvalue_3))
  (Default|CallSpawnedThirdPerson _output_get))

(event EventBeginPlay
  (bind _array (Utilities|Array|MakeArray "android.permission.WRITE_EXTERNAL_STORAGE" "android.permission.READ_EXTERNAL_STORAGE" "com.oculus.permission.USE_SCENE"))
  ;[1 1 1] Checks for permissions
  (for (_array_element _array_index) _array
    (bind _returnvalue (Class|AndroidPermissionFunctionLibrary|CheckPermission _array_element))
    (if _returnvalue
      (bind _returnvalue_2 (Utilities|Array|Add (Variables|Default|GetNumberOfPermissionsGranted) _array_index))
      (Development|PrintString (Utilities|String|ToString(Integer) _returnvalue_2))
      (if (== _returnvalue_2 2)
        (Development|PrintString "Has all permissions")
        (Utilities|FlowControl|Delay 1.0)
        (CallFunction|SpawnMainMenu)
        (else
          (Development|PrintString "Failed to request permissions")
          (Default|CallFailedPermissions)))
      (else
        (bind _returnvalue_3 (Class|AndroidPermissionFunctionLibrary|AcquirePermissions _array))
        (EventDispatchers|BindEventtoOnPermissionsGrantedDynamicDelegate _returnvalue_3 (delegate Custom|PermissionGrantedResult))))))