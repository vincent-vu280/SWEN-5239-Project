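; BP_PermissionsCube is a mixed-reality actor that shows permission status on a cube and starts the project session.
; BeginPlay registers a permissions-granted callback with ACGameManager; when it fires, the cube changes material and, after a short delay, BeginProjectSession is called.
; A failure handler switches the cube to a red-only material, but its registration node is disconnected, so it is never bound.
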(event Custom|HasPermissions_Event
  (Rendering|Material|SetMaterial (Variables|Default|GetCube) 0 "/Engine/MapTemplates/Materials/BasicAsset03.BasicAsset03")
  (Utilities|FlowControl|Delay 2.0)
  (Default|BeginProjectSession (Variables|Default|GetAC_GameManager)))

(event Custom|FailedPermissions_Event
  (Rendering|Material|SetMaterial (Variables|Default|GetCube) 0 "/Engine/EngineDebugMaterials/VertexColorViewMode_RedOnly.VertexColorViewMode_RedOnly"))

(event EventBeginPlay
  (EventDispatchers|AssignHasPermissions (Variables|Default|GetAC_GameManager) (delegate Custom|HasPermissions_Event)))

(event Collision|EventActorBeginOverlap
  (params (OtherActor :type Actor%20Object%20Reference)))

(event EventTick
  (params (DeltaSeconds :type Float%20%28single-precision%29)))

(fn ConstructionScript)